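; Tablet is an interactable pickup actor that shows a subtitle widget when the player interacts with it.
; Its capsule overlap events message the overlapping actor on entering and leaving the interact area, passing itself on entry.
; DoInterract destroys the actor first, then adds Subtitle1 to the screen, with a one-second delay before a debug print and widget removal on the already destroyed actor.
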(event OnComponentBeginOverlap(Capsule)
  (params (OverlappedComponent :type Primitive%20Component%20Object%20Reference) (OtherActor :type Actor%20Object%20Reference) (OtherComp :type Primitive%20Component%20Object%20Reference) (OtherBodyIndex :type Integer) (bFromSweep :type Boolean) (SweepResult :type Hit%20Result%20Structure%20%28by%20ref%29))
  (Class|InteractActorInterface|EnterInterractArea(Message) OtherActor self))

(event OnComponentEndOverlap(Capsule)
  (params (OverlappedComponent :type Primitive%20Component%20Object%20Reference) (OtherActor :type Actor%20Object%20Reference) (OtherComp :type Primitive%20Component%20Object%20Reference) (OtherBodyIndex :type Integer))
  (Class|InteractActorInterface|ExitInterractArea(Message) OtherActor))

(event EventDoInterract
  (Actor|DestroyActor)
  (bind _returnvalue (UserInterface|CreateWidget "/Game/UI/Subtitles/subtitle1.subtitle1_C"))
  (UserInterface|Viewport|AddtoPlayerScreen _returnvalue)
  (Utilities|FlowControl|Delay 1.0)
  (Development|PrintString "eiei")
  (Widget|RemovefromParent _returnvalue))

(event EventBeginPlay
  (bind _asbp_first_person_character (Utilities|Casting|CastToBP_FirstPersonCharacter (Game|GetPlayerCharacter 0)))
  (Variables|Default|Setplayer _asbp_first_person_character))

(fn ConstructionScript)